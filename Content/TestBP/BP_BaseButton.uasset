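; Base pushable button actor that makes its connected spawner spawn a turtle when the player presses Interact nearby.
; Collision box overlaps with the third-person character toggle the actor's input, though both begin and end overlap set IsPushable to true.
; A timeline lerps the button inward with a click sound, then after a short delay it triggers the spawner and its sound while a second timeline returns the button.
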(event `self.ReceiveBeginPlay`
  (bind (_returnvalue_location _returnvalue_rotation _returnvalue_scale) (`KismetMathLibrary.BreakTransform` (`SceneComponent.GetRelativeTransform` (`self.Button`))))
  (set `self.Out position` (`KismetMathLibrary.MakeTransform` _returnvalue_location _returnvalue_rotation _returnvalue_scale))
  (set `self.In position` (`KismetMathLibrary.MakeTransform` (- _returnvalue_location (-4.0 0.0 0.0)) _returnvalue_rotation _returnvalue_scale)))

(event `InputAction|Interact`
  (params (Key :type "Key Structure"))
  (bind _returnvalue (`self.K2_GetActorLocation`))
  (:`Pressed`
    (if (`self.Is pushable`)
      ;[1 1 1] button animation
      (`GameplayStatics.PlaySoundAtLocation` "/Engine/VREditor/Sounds/UI/Click_on_Button_Cue.Click_on_Button_Cue" _returnvalue (struct) 1.0 1.0 0.0 null null null)
      (bind (_direction _button_in) (`Timeline|Button In` :!via `PlayFromStart`)
        (:`Update`
          (`SceneComponent.K2_SetRelativeTransform` (`self.Button`) (`KismetMathLibrary.TLerp` (`self.Out position`) (`self.In position`) _button_in) false false))
        (:`Finished`
          (`KismetSystemLibrary.Delay` 0.5)
          ;[1 1 1] move play sound inside turtle code
          (`BaseSpawner.SpawnTurtle` (`self.Connected Spawner`))
          (`GameplayStatics.PlaySoundAtLocation` "/Game/TestSound/spawn_sound.spawn_sound" (`self.K2_GetActorLocation` (`self.Connected Spawner`)) (struct) 1.0 1.0 0.0 null null null)
          (bind (_direction_2 _button_in_2) (`Timeline|Button Out` :!via `ReverseFromEnd`)
            (:`Update`
              (`SceneComponent.K2_SetRelativeTransform` (`self.Button`) (`KismetMathLibrary.TLerp` (`self.Out position`) (`self.In position`) _button_in_2) false false)))))
      (else
        (`GameplayStatics.PlaySoundAtLocation` "/Engine/VREditor/Sounds/UI/Click_on_Button.Click_on_Button" _returnvalue (struct) 1.0 1.0 0.0 null null null)))))

(event `self.CollisionBox.OnComponentBeginOverlap`
  (params (OverlappedComponent :type "PrimitiveComponent Object Reference") (OtherActor :type "Actor Object Reference") (OtherComp :type "PrimitiveComponent Object Reference") (OtherBodyIndex :type Integer) (bFromSweep :type Boolean) (SweepResult :type "HitResult Structure (by ref)"))
  ;[1 1 1] enable input when actor is close
  (cast `/Game/ThirdPersonBP/Blueprints/ThirdPersonCharacter` OtherActor)
  (`self.EnableInput` (`GameplayStatics.GetPlayerController` 0))
  (set `self.Is pushable` true))

(event `self.CollisionBox.OnComponentEndOverlap`
  (params (OverlappedComponent :type "PrimitiveComponent Object Reference") (OtherActor :type "Actor Object Reference") (OtherComp :type "PrimitiveComponent Object Reference") (OtherBodyIndex :type Integer))
  ;[1 1 1] disable input when actor is too far
  (cast `/Game/ThirdPersonBP/Blueprints/ThirdPersonCharacter` OtherActor)
  (`self.DisableInput` (`GameplayStatics.GetPlayerController` 0))
  (set `self.Is pushable` true))

(fn `UserConstructionScript`)